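; BP-Cube is a physics-driven player cube that moves along the Y axis, jumps and fast-falls.
; Axis inputs apply velocity-change impulses, with jumping gated by a Floored flag set from upward hit normals.
; The Static action disables physics and locks movement when floored below a Y-velocity threshold, restoring both on release.
; Tick clamps Y velocity in both directions, while the fall-speed clamp is disconnected and never runs.
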(event `InputAction|Static`
  (params (Key :type "Key Structure"))
  ;[1 1 1] Static
  (:`Pressed`
    (bind _y (`self.Get Y Velocity`))
    (if (< _y (`self.StaticMaxSpeed`))
      (if (`self.Floored`)
        (set `self.Cube Physics Lock` true)
        (`PrimitiveComponent.SetSimulatePhysics` (`self.Cube`) false))))
  (:`Released`
    (`PrimitiveComponent.SetSimulatePhysics` (`self.Cube`) true)
    (set `self.Cube Physics Lock` false)))

(event `self.ReceiveTick`
  (params (DeltaSeconds :type "Float (single-precision)"))
  ;[1 0 0.01989] Event Tick
  (`self.Tick 1`)
  (`self.Tick 2`)
  (`self.Tick 3`))

(event `Tick 2`
  (bind _returnvalue (* (`self.MaxSpeed`) -1.0))
  ;[1 0.2814 0] Max Speed
  (bind _y (`self.Get Y Velocity`))
  (if (< _y _returnvalue)
    (bind _returnvalue_2 (`PrimitiveComponent.GetPhysicsLinearVelocity` (`self.Cube`) "None"))
    (`PrimitiveComponent.SetPhysicsLinearVelocity` (`self.Cube`) (`KismetMathLibrary.MakeVector` (.x _returnvalue_2) _returnvalue (.z _returnvalue_2)) false "None")))

(event `Tick 1`
  ;[1 0.2814 0] Max Speed
  (bind _y (`self.Get Y Velocity`))
  (if (> _y (`self.MaxSpeed`))
    (bind _returnvalue (`PrimitiveComponent.GetPhysicsLinearVelocity` (`self.Cube`) "None"))
    (`PrimitiveComponent.SetPhysicsLinearVelocity` (`self.Cube`) (`KismetMathLibrary.MakeVector` (.x _returnvalue) (`self.MaxSpeed`) (.z _returnvalue)) false "None")))

(event `InputAxis|Right`
  (params (AxisValue :type "Float (single-precision)"))
  ;[0.2889 0.3106 1] Movement
  (if (not (`self.Cube Physics Lock`))
    (`PrimitiveComponent.AddImpulse` (`self.Cube`) (`KismetMathLibrary.MakeVector` 0.0 (* AxisValue (`self.Speed`))) "None" true)))

(event `InputAxis|Left`
  (params (AxisValue :type "Float (single-precision)"))
  ;[0.2889 0.3106 1] Movement
  (if (not (`self.Cube Physics Lock`))
    (`PrimitiveComponent.AddImpulse` (`self.Cube`) (`KismetMathLibrary.MakeVector` 0.0 (* AxisValue (`self.Speed`))) "None" true)))

(event `InputAxis|Up`
  (params (AxisValue :type "Float (single-precision)"))
  ;[0.165 1 0.3104] Jumping
  (if (`self.Floored`)
    (set `self.Floored` false)
    (if (not (`self.Cube Physics Lock`))
      (`PrimitiveComponent.AddImpulse` (`self.Cube`) (`KismetMathLibrary.MakeVector` 0.0 0.0 (* AxisValue (`self.JumpForce`))) "None" true))))

(event `self.ReceiveHit`
  (params (MyComp :type "PrimitiveComponent Object Reference") (Other :type "Actor Object Reference") (OtherComp :type "PrimitiveComponent Object Reference") (bSelfMoved :type Boolean) (HitLocation :type "Vector Structure") (HitNormal :type "Vector Structure") (NormalImpulse :type "Vector Structure") (Hit :type "HitResult Structure (by ref)"))
  ;[1 0.09783 0.9804] Floored
  (set `self.Floored` (== HitNormal (`KismetMathLibrary.Vector_Up`))))

(event `InputAxis|Down`
  (params (AxisValue :type "Float (single-precision)"))
  ;[1 0.9337 0] Fast Fall
  (if (not (`self.Cube Physics Lock`))
    (bind _returnvalue (`PrimitiveComponent.GetPhysicsLinearVelocity` (`self.Cube`) "None"))
    (if (<= (.z _returnvalue) 0.0)
      (`PrimitiveComponent.AddImpulse` (`self.Cube`) (`KismetMathLibrary.MakeVector` 0.0 0.0 (* AxisValue (`self.FastFallSpeed`))) "None" true))))

(event `Tick 3`
  ;[1 1 1] Fall Max Speed
  (bind _returnvalue (`PrimitiveComponent.GetPhysicsLinearVelocity` (`self.Cube`) "None")))

(fn `Get Y Velocity`
  (returns (Y :type "Float (double-precision)"))
  (bind _returnvalue (`PrimitiveComponent.GetPhysicsLinearVelocity` (`self.Cube`) "None"))
  (return (.y _returnvalue)))

(fn `UserConstructionScript`)